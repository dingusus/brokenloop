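; BP_enemy1 is a ranged enemy that chases and shoots at the player and can be dazed by a lantern.
; Two overlap volumes set sight and shooting range; Tick moves it along X only toward a seen player.
; In shooting range it stops and, through a Delay on Tick, spawns an actor aimed at the player every two seconds.
; inLantern halts both behaviors; exitLantern clears the daze after a delay.
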(event OnComponentBeginOverlap(seePlayerRange)
  (params (OverlappedComponent :type Primitive%20Component%20Object%20Reference) (OtherActor :type Actor%20Object%20Reference) (OtherComp :type Primitive%20Component%20Object%20Reference) (OtherBodyIndex :type Integer) (bFromSweep :type Boolean) (SweepResult :type Hit%20Result%20Structure%20%28by%20ref%29))
  (bind _asbp_third_person_character (Utilities|Casting|CastToBP_ThirdPersonCharacter OtherActor))
  (Variables|Default|SetplayerReference _asbp_third_person_character)
  (Variables|Default|SetcanSeePlayer true))

(event OnComponentBeginOverlap(canShootRange)
  (params (OverlappedComponent :type Primitive%20Component%20Object%20Reference) (OtherActor :type Actor%20Object%20Reference) (OtherComp :type Primitive%20Component%20Object%20Reference) (OtherBodyIndex :type Integer) (bFromSweep :type Boolean) (SweepResult :type Hit%20Result%20Structure%20%28by%20ref%29))
  (bind _asbp_third_person_character (Utilities|Casting|CastToBP_ThirdPersonCharacter OtherActor))
  (Variables|Default|SetplayerReference _asbp_third_person_character)
  (Variables|Default|SetcanShootPlayer true))

(event OnComponentEndOverlap(canShootRange)
  (params (OverlappedComponent :type Primitive%20Component%20Object%20Reference) (OtherActor :type Actor%20Object%20Reference) (OtherComp :type Primitive%20Component%20Object%20Reference) (OtherBodyIndex :type Integer))
  (bind _asbp_third_person_character (Utilities|Casting|CastToBP_ThirdPersonCharacter OtherActor))
  (Variables|Default|SetplayerReference _asbp_third_person_character)
  (Variables|Default|SetcanShootPlayer false))

(event OnComponentEndOverlap(seePlayerRange)
  (params (OverlappedComponent :type Primitive%20Component%20Object%20Reference) (OtherActor :type Actor%20Object%20Reference) (OtherComp :type Primitive%20Component%20Object%20Reference) (OtherBodyIndex :type Integer))
  (bind _asbp_third_person_character (Utilities|Casting|CastToBP_ThirdPersonCharacter OtherActor))
  (Variables|Default|SetplayerReference _asbp_third_person_character)
  (Variables|Default|SetcanSeePlayer false))

(event Custom|inLantern
  (Variables|Default|SetisDazed true)
  (Development|PrintString "set is dazed"))

(event Custom|exitLantern
  (Utilities|FlowControl|Delay 3.0)
  (Variables|Default|SetisDazed false)
  (Development|PrintString "undazed"))

(event EventTick
  (params (DeltaSeconds :type Float%20%28single-precision%29))
  (bind _returnvalue (Transformation|GetActorLocation))
  (if (not (Variables|Default|GetisDazed))
    (if (Variables|Default|GetcanSeePlayer)
      (if (Variables|Default|GetcanShootPlayer)
        (Utilities|FlowControl|Delay 2.0)
        (if (not (Variables|Default|GetisDazed))
          (Game|SpawnActorfromClass "/Game/CONTENT/PROTOTYPE/blueprint/Enemies/enemy1/BP_enemy1Projectile.BP_enemy1Projectile_C" (Math|Transform|MakeTransform (Transformation|GetActorLocation) (Math|Rotator|FindLookatRotation (Transformation|GetActorLocation) (Transformation|GetActorLocation (Variables|Default|GetplayerReference))) "2.000000,2.000000,2.000000") "AlwaysSpawn" "MultiplyWithRoot" 0 0)
          (Development|PrintString "shooting"))
        (else
          (Transformation|SetActorLocation (Math|Vector|MakeVector (+ (* (* (Math|Float|Sign(Float) (- (.x (Transformation|GetActorLocation (Variables|Default|GetplayerReference))) (.x (Transformation|GetActorLocation)))) (Variables|Default|GetmovementSpeed)) (Utilities|Time|GetWorldDeltaSeconds)) (.x _returnvalue)) (.y _returnvalue) (.z _returnvalue)) false false))))))

(event EventBeginPlay
  (bind _asbp_third_person_character (Utilities|Casting|CastToBP_ThirdPersonCharacter (Game|GetPlayerCharacter 0)))
  (Variables|Default|SetplayerReference _asbp_third_person_character))

(fn ConstructionScript)