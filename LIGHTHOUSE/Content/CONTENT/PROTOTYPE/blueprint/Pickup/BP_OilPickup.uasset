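; BP_OilPickup is a collectible that refills the player's oil when walked into.
; On BeginPlay it caches the player as a BP_ThirdPersonCharacter.
; When the player overlaps its Collision component, it adds a fixed amount to OilAmount in the player's SaveRef, caps it at a maximum, then destroys itself.
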(event OnComponentBeginOverlap(Collision)
  (params (OverlappedComponent :type Primitive%20Component%20Object%20Reference) (OtherActor :type Actor%20Object%20Reference) (OtherComp :type Primitive%20Component%20Object%20Reference) (OtherBodyIndex :type Integer) (bFromSweep :type Boolean) (SweepResult :type Hit%20Result%20Structure%20%28by%20ref%29))
  (bind _playerref (Variables|Default|GetPlayerRef))
  (bind _saveref (Variables|/Game/ThirdPerson/Blueprints/BP_ThirdPersonCharacter.BP_ThirdPersonCharacter_C|GetSaveRef _playerref))
  (if (== OtherActor _playerref)
    (Variables|/Game/CONTENT/PROTOTYPE/PlayerStats.PlayerStats_C|SetOilAmount _saveref (+ (Variables|/Game/CONTENT/PROTOTYPE/PlayerStats.PlayerStats_C|GetOilAmount _saveref) 2.0))
    (if (>= (Variables|/Game/CONTENT/PROTOTYPE/PlayerStats.PlayerStats_C|GetOilAmount _saveref) 2e+01)
      (Variables|/Game/CONTENT/PROTOTYPE/PlayerStats.PlayerStats_C|SetOilAmount _saveref 2e+01))
    (Actor|DestroyActor)))

(event EventBeginPlay
  (bind _asbp_third_person_character (Utilities|Casting|CastToBP_ThirdPersonCharacter (Game|GetPlayerCharacter 0)))
  (Variables|Default|SetPlayerRef _asbp_third_person_character))

(fn ConstructionScript)