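; BP_ShatteredMemory is a pickup that hands the player a story memory when touched.
; On BeginPlay it caches the player's BP_ThirdPersonCharacter reference.
; When that player overlaps its Collision component, it sets CurrentMemory from the character's MemoriesList using MemoryID, calls SetMemoryText to refresh the text, then destroys itself.
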(event OnComponentBeginOverlap(Collision)
  (params (OverlappedComponent :type Primitive%20Component%20Object%20Reference) (OtherActor :type Actor%20Object%20Reference) (OtherComp :type Primitive%20Component%20Object%20Reference) (OtherBodyIndex :type Integer) (bFromSweep :type Boolean) (SweepResult :type Hit%20Result%20Structure%20%28by%20ref%29))
  (bind _playerref (Variables|Default|GetPlayerRef))
  (if (== OtherActor _playerref)
    (Variables|/Game/ThirdPerson/Blueprints/BP_ThirdPersonCharacter.BP_ThirdPersonCharacter_C|SetCurrentMemory _playerref (Utilities|Array|Get(acopy) (Variables|/Game/ThirdPerson/Blueprints/BP_ThirdPersonCharacter.BP_ThirdPersonCharacter_C|GetMemoriesList _playerref) (Variables|Default|GetMemoryID)))
    (Default|SetMemoryText _playerref)
    (Actor|DestroyActor)))

(event EventBeginPlay
  (bind _asbp_third_person_character (Utilities|Casting|CastToBP_ThirdPersonCharacter (Game|GetPlayerCharacter 0)))
  (Variables|Default|SetPlayerRef _asbp_third_person_character))

(fn ConstructionScript)