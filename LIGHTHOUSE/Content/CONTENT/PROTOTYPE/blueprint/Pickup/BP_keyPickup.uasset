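; Key pickup actor that grants the third-person player character one of three keys, chosen by its KeyType.
; When its HitBox overlaps the character, it sets the matching HasKey flag on that character, prints a message and destroys itself.
; BeginPlay switches on KeyType, but none of its branches does anything.
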(event OnComponentBeginOverlap(hitBox)
  (params (OverlappedComponent :type Primitive%20Component%20Object%20Reference) (OtherActor :type Actor%20Object%20Reference) (OtherComp :type Primitive%20Component%20Object%20Reference) (OtherBodyIndex :type Integer) (bFromSweep :type Boolean) (SweepResult :type Hit%20Result%20Structure%20%28by%20ref%29))
  (bind _asbp_third_person_character (Utilities|Casting|CastToBP_ThirdPersonCharacter OtherActor))
  (Variables|Default|SetplayerCharacterReference _asbp_third_person_character)
  (switch Utilities|FlowControl|Switch|SwitchonKeys (Variables|Default|GetkeyType)
    (:NewEnumerator0
      (Variables|/Game/ThirdPerson/Blueprints/BP_ThirdPersonCharacter.BP_ThirdPersonCharacter_C|SethasKey1? (Variables|Default|GetplayerCharacterReference) true)
      (Development|PrintString "picked up key 1"))
    (:NewEnumerator1
      (Variables|/Game/ThirdPerson/Blueprints/BP_ThirdPersonCharacter.BP_ThirdPersonCharacter_C|SethasKey2? (Variables|Default|GetplayerCharacterReference) true)
      (Development|PrintString "picked up key 2"))
    (:NewEnumerator2
      (Variables|/Game/ThirdPerson/Blueprints/BP_ThirdPersonCharacter.BP_ThirdPersonCharacter_C|SethasKey3? (Variables|Default|GetplayerCharacterReference) true)
      (Development|PrintString "picked up key 3")))
  (Actor|DestroyActor))

(event EventBeginPlay
  (switch Utilities|FlowControl|Switch|SwitchonKeys (Variables|Default|GetkeyType)))

(event Collision|EventActorBeginOverlap
  (params (OtherActor :type Actor%20Object%20Reference)))

(event EventTick
  (params (DeltaSeconds :type Float%20%28single-precision%29)))

(fn ConstructionScript)