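; BP_Checkpoint is a checkpoint that records a respawn-style location on the player's controller when the player character touches it.
; On BeginPlay it caches its root world location and references to the first player's BP_ThirdPersonPlayerController and BP_ThirdPersonCharacter.
; When that character overlaps the Box, it writes the location to the controller's CtrlCheckpointLocation and swaps the Cube material to MI_ThirdPersonColWay.
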(event OnComponentBeginOverlap(Box)
  (params (OverlappedComponent :type Primitive%20Component%20Object%20Reference) (OtherActor :type Actor%20Object%20Reference) (OtherComp :type Primitive%20Component%20Object%20Reference) (OtherBodyIndex :type Integer) (bFromSweep :type Boolean) (SweepResult :type Hit%20Result%20Structure%20%28by%20ref%29))
  (if (== OtherActor (Variables|Default|GetPlayerRef))
    (Variables|/Game/ThirdPerson/Blueprints/BP_ThirdPersonPlayerController.BP_ThirdPersonPlayerController_C|SetCtrlCheckpointLocation (Variables|Default|GetControllerRef) (Variables|Default|GetCheckpointLocation))
    (Rendering|Material|SetMaterial (Variables|Default|GetCube) 0 "/Game/ThirdPerson/MI_ThirdPersonColWay.MI_ThirdPersonColWay")))

(event EventBeginPlay
  (Variables|Default|SetCheckpointLocation (Transformation|GetWorldLocation (Variables|Default|GetDefaultSceneRoot)))
  (bind _asbp_third_person_player_controller (Utilities|Casting|CastToBP_ThirdPersonPlayerController (Game|GetPlayerController 0)))
  (Variables|Default|SetControllerRef _asbp_third_person_player_controller)
  (bind _asbp_third_person_character (Utilities|Casting|CastToBP_ThirdPersonCharacter (Game|GetPlayerCharacter 0)))
  (Variables|Default|SetPlayerRef _asbp_third_person_character))

(fn ConstructionScript)