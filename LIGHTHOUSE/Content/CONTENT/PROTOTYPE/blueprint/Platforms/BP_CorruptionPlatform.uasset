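; Corruption platform that slows the player and disables their lantern while they stand in its box trigger.
; On overlap, a looping timer runs CheckCorrupted, which lowers walk speed, makes LanternCollision ignore a trace channel and hides the player's Sphere.
; Leaving clears the touch flag and pauses the timer shortly after, letting a final check restore speed, collision and visibility after a few seconds' delay.
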(event OnComponentBeginOverlap(Box)
  (params (OverlappedComponent :type Primitive%20Component%20Object%20Reference) (OtherActor :type Actor%20Object%20Reference) (OtherComp :type Primitive%20Component%20Object%20Reference) (OtherBodyIndex :type Integer) (bFromSweep :type Boolean) (SweepResult :type Hit%20Result%20Structure%20%28by%20ref%29))
  (if (== OtherActor (Variables|Default|GetPlayerRef))
    (Variables|Default|SetIsTouching true)
    (bind _returnvalue (Utilities|Time|SetTimerbyEvent (delegate Custom|CheckCorrupted) 0.1 true))))

(event OnComponentEndOverlap(Box)
  (params (OverlappedComponent :type Primitive%20Component%20Object%20Reference) (OtherActor :type Actor%20Object%20Reference) (OtherComp :type Primitive%20Component%20Object%20Reference) (OtherBodyIndex :type Integer))
  (if (== OtherActor (Variables|Default|GetPlayerRef))
    (Variables|Default|SetIsTouching false)
    (Utilities|FlowControl|Delay 0.5)
    (Utilities|Time|PauseTimerbyHandle (stale OnComponentBeginOverlap(Box) _returnvalue))))

(event Custom|CheckCorrupted
  (bind _playerref (Variables|Default|GetPlayerRef))
  (bind _lanterncollision (Variables|/Game/ThirdPerson/Blueprints/BP_ThirdPersonCharacter.BP_ThirdPersonCharacter_C|GetLanternCollision _playerref))
  (bind _sphere (Variables|/Game/ThirdPerson/Blueprints/BP_ThirdPersonCharacter.BP_ThirdPersonCharacter_C|GetSphere _playerref))
  (bind _charactermovement (Variables|/Script/Engine.Character|GetCharacterMovement _playerref))
  (if (Variables|Default|GetIsTouching)
    (Variables|/Script/Engine.CharacterMovementComponent|SetMaxWalkSpeed _charactermovement 2.5e+02)
    (Collision|SetCollisionResponsetoChannel _lanterncollision "ECC_GameTraceChannel1" "ECR_Ignore")
    (Utilities|FlowControl|Delay 0.1)
    (Development|SetHiddeninGame _sphere true false)
    (else
      (Utilities|FlowControl|Delay 3.0)
      (Variables|/Script/Engine.CharacterMovementComponent|SetMaxWalkSpeed _charactermovement (Variables|Default|GetInitialSpeed))
      (Collision|SetCollisionResponsetoChannel _lanterncollision "ECC_GameTraceChannel1" "ECR_Overlap")
      (Development|SetHiddeninGame _sphere false false))))

(event EventBeginPlay
  (bind _asbp_third_person_character (Utilities|Casting|CastToBP_ThirdPersonCharacter (Game|GetPlayerCharacter 0)))
  (bind _output_get (Variables|Default|SetPlayerRef _asbp_third_person_character))
  (Variables|Default|SetInitialSpeed (Variables|/Script/Engine.CharacterMovementComponent|GetMaxWalkSpeed (Variables|/Script/Engine.Character|GetCharacterMovement _output_get))))

(fn ConstructionScript)