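; A platform that falls away shortly after the player steps on it.
; BeginPlay caches the player character as BP_ThirdPersonCharacter, and the Box overlap reacts only to that actor.
; The first such overlap passes a DoOnce, waits briefly, enables physics simulation on both the Cube and Box, then destroys the actor after a further delay.
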(event OnComponentBeginOverlap(Box)
  (params (OverlappedComponent :type Primitive%20Component%20Object%20Reference) (OtherActor :type Actor%20Object%20Reference) (OtherComp :type Primitive%20Component%20Object%20Reference) (OtherBodyIndex :type Integer) (bFromSweep :type Boolean) (SweepResult :type Hit%20Result%20Structure%20%28by%20ref%29))
  (if (== OtherActor (Variables|Default|GetPlayerRef))
    (Utilities|FlowControl|DoOnce false
      (:Completed
        (Utilities|FlowControl|Delay 1.0)
        (Physics|SetSimulatePhysics (Variables|Default|GetCube) true)
        (Utilities|FlowControl|Delay 3.0)
        (Actor|DestroyActor)))))

(event EventBeginPlay
  (bind _asbp_third_person_character (Utilities|Casting|CastToBP_ThirdPersonCharacter (Game|GetPlayerCharacter 0)))
  (Variables|Default|SetPlayerRef _asbp_third_person_character))

(fn ConstructionScript)