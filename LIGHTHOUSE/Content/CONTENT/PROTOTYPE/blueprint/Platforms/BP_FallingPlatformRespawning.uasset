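; A prototype platform that falls after the player character steps on it, then respawns at its original position.
; BeginPlay caches the player reference and the starting locations of the Cube mesh and Box trigger.
; Player overlap fires a DoOnce that, after short delays, enables physics on both components, then hides them and disables collision.
; RespawnPlatform immediately restores location, visibility and collision, stops physics and resets the DoOnce for reuse.
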(event OnComponentBeginOverlap(Box)
  (params (OverlappedComponent :type Primitive%20Component%20Object%20Reference) (OtherActor :type Actor%20Object%20Reference) (OtherComp :type Primitive%20Component%20Object%20Reference) (OtherBodyIndex :type Integer) (bFromSweep :type Boolean) (SweepResult :type Hit%20Result%20Structure%20%28by%20ref%29))
  (bind _cube (Variables|Default|GetCube))
  (if (== OtherActor (Variables|Default|GetPlayerRef))
    (Utilities|FlowControl|DoOnce false
      (:Completed
        (if (not (Variables|Default|GetHasFallen))
          (Utilities|FlowControl|Delay 1.0)
          (Physics|SetSimulatePhysics _cube true)
          (Variables|Default|SetHasFallen true)
          (Utilities|FlowControl|Delay 3.0)
          (Rendering|SetVisibility _cube false false)
          (Collision|SetCollisionResponsetoAllChannels _cube "ECR_Ignore")
          (CallFunction|RespawnPlatform))))))

(event Custom|RespawnPlatform
  (bind _cube (Variables|Default|GetCube))
  (bind _cube_2 (Variables|Default|GetCube))
  (bind _box (Variables|Default|GetBox))
  (Physics|SetSimulatePhysics _box false)
  (Transformation|SetWorldLocationAndRotation _cube_2 (Variables|Default|GetPlatformLocation) "0, 0, 0" false false)
  (Transformation|SetWorldLocationAndRotation _box (Variables|Default|GetCollisionLocation) "0, 0, 0" false false)
  (Rendering|SetVisibility _cube_2 true false)
  (Collision|SetCollisionResponsetoAllChannels _cube_2 "ECR_Block")
  (Collision|SetCollisionResponsetoAllChannels _box "ECR_Overlap")
  (Variables|Default|SetHasFallen false)
  (Utilities|FlowControl|DoOnce false) ; enters at Reset
)

(event EventBeginPlay
  (bind _asbp_third_person_character (Utilities|Casting|CastToBP_ThirdPersonCharacter (Game|GetPlayerCharacter 0)))
  (Variables|Default|SetPlayerRef _asbp_third_person_character)
  (Variables|Default|SetPlatformLocation (Transformation|GetWorldLocation (Variables|Default|GetCube)))
  (Variables|Default|SetCollisionLocation (Transformation|GetWorldLocation (Variables|Default|GetBox))))

(fn ConstructionScript)