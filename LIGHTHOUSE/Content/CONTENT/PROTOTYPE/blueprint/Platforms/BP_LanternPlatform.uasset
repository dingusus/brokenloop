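; BP_LanternPlatform is a prototype platform that becomes visible and solid only while something overlaps its Box trigger.
; Box overlap begin unhides the Cube and enables query and physics collision, and overlap end hides it and disables collision.
; BeginPlay stores a reference to the third-person character and turns Cube collision off.
; The overlap events do not filter the overlapping actor or use that stored reference.
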(event OnComponentBeginOverlap(Box)
  (params (OverlappedComponent :type Primitive%20Component%20Object%20Reference) (OtherActor :type Actor%20Object%20Reference) (OtherComp :type Primitive%20Component%20Object%20Reference) (OtherBodyIndex :type Integer) (bFromSweep :type Boolean) (SweepResult :type Hit%20Result%20Structure%20%28by%20ref%29))
  (bind _cube (Variables|Default|GetCube))
  (Development|SetHiddeninGame _cube false false)
  (Collision|SetCollisionEnabled _cube "QueryAndPhysics"))

(event OnComponentEndOverlap(Box)
  (params (OverlappedComponent :type Primitive%20Component%20Object%20Reference) (OtherActor :type Actor%20Object%20Reference) (OtherComp :type Primitive%20Component%20Object%20Reference) (OtherBodyIndex :type Integer))
  (bind _cube (Variables|Default|GetCube))
  (Development|SetHiddeninGame _cube true false)
  (Collision|SetCollisionEnabled _cube "NoCollision"))

(event EventBeginPlay
  (bind _asbp_third_person_character (Utilities|Casting|CastToBP_ThirdPersonCharacter (Game|GetPlayerCharacter 0)))
  (Variables|Default|SetPlayerRef _asbp_third_person_character)
  (Collision|SetCollisionEnabled (Variables|Default|GetCube) "NoCollision"))

(fn ConstructionScript)