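; Prototype platform actor that turns its cube into a hallucination when the player's sanity threshold flag is set.
; A two-second looping timer polls that flag on the third-person character.
; When set, it applies the character's hallucination material to the cube and clears the flag, with no revert here.
; A FlipFlop then alternates between setting the character's stage 1 and stage 2 sanity flags, calling its Sanity function each time.
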(event Custom|switchmaterial
  (bind _asbp_third_person_character (Utilities|Casting|CastToBP_ThirdPersonCharacter (Game|GetPlayerCharacter 0)))
  (if (Variables|/Game/ThirdPerson/Blueprints/BP_ThirdPersonCharacter.BP_ThirdPersonCharacter_C|Getsanitythreshold _asbp_third_person_character)
    (Rendering|Material|SetMaterial (Variables|Default|GetCube) 0 (Variables|/Game/ThirdPerson/Blueprints/BP_ThirdPersonCharacter.BP_ThirdPersonCharacter_C|Gethallucination_material _asbp_third_person_character))
    (Variables|/Game/ThirdPerson/Blueprints/BP_ThirdPersonCharacter.BP_ThirdPersonCharacter_C|Setsanitythreshold _asbp_third_person_character false)
    (Utilities|FlowControl|FlipFlop
      (:A
        (Variables|/Game/ThirdPerson/Blueprints/BP_ThirdPersonCharacter.BP_ThirdPersonCharacter_C|Setstage1?_sanity _asbp_third_person_character true)
        (Default|Sanity _asbp_third_person_character))
      (:B
        (Variables|/Game/ThirdPerson/Blueprints/BP_ThirdPersonCharacter.BP_ThirdPersonCharacter_C|Setstage2?_sanity _asbp_third_person_character true)
        (Default|Sanity _asbp_third_person_character)))))

(event EventBeginPlay
  (Utilities|Time|SetTimerbyEvent (delegate Custom|switchmaterial) 2.0 true))

(fn ConstructionScript)