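; Camera actor Blueprint that smoothly follows a target actor.
; Every Tick, Updatecamera interpolates its location toward the target's position plus an offset along the target's forward vector, using VInterpTo.
; The offset drops its Y component, so only X and Z shift with facing, and a LockHeight flag keeps the camera's current height as the base instead of the target's.
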(event EventBeginPlay)

(event Collision|EventActorBeginOverlap
  (params (OtherActor :type Actor%20Object%20Reference)))

(event EventTick
  (params (DeltaSeconds :type Float%20%28single-precision%29))
  (CallFunction|Updatecamera))

(fn ConstructionScript)

(fn Updatecamera
  (bind _follow_target (Variables|Default|Getfollow_target))
  (bind _follow_target_2 (Variables|Default|Getfollow_target))
  (bind _cameraoffset (Variables|Default|Getcameraoffset))
  (bind _returnvalue (Transformation|GetActorForwardVector _follow_target_2))
  (bind _returnvalue_2 (Transformation|GetActorLocation _follow_target))
  (bind _returnvalue_3 (* _returnvalue _cameraoffset))
  (Transformation|SetActorLocation (Math|Interpolation|VInterpTo (Transformation|GetActorLocation) (+ (Math|Vector|MakeVector (.x _returnvalue_2) (.y _returnvalue_2) (select (Variables|Default|Getlock%20height) (.z (Transformation|GetActorLocation)) (.z _returnvalue_2))) (Math|Vector|MakeVector (.x _returnvalue_3) 0.0 (.z _returnvalue_3))) (Utilities|Time|GetWorldDeltaSeconds) (Variables|Default|GetInterp%20Speed)) false false))