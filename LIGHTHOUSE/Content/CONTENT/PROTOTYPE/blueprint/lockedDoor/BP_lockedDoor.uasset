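; BP_lockedDoor is a prototype door that opens for a player character holding the matching key.
; On box overlap by BP_ThirdPersonCharacter, it switches on LockType and checks that character's HasKey1, HasKey2 or HasKey3 flag.
; With the right key, the door snaps 1000 units along negative X from the relative location saved at BeginPlay, with no animation or closing logic.
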(event OnComponentBeginOverlap(Box)
  (params (OverlappedComponent :type Primitive%20Component%20Object%20Reference) (OtherActor :type Actor%20Object%20Reference) (OtherComp :type Primitive%20Component%20Object%20Reference) (OtherBodyIndex :type Integer) (bFromSweep :type Boolean) (SweepResult :type Hit%20Result%20Structure%20%28by%20ref%29))
  (bind _doorlocation (Variables|Default|GetdoorLocation))
  (bind _asbp_third_person_character (Utilities|Casting|CastToBP_ThirdPersonCharacter OtherActor))
  (Variables|Default|SetplayerRef _asbp_third_person_character)
  (switch Utilities|FlowControl|Switch|SwitchonKeys (Variables|Default|GetlockType)
    (:NewEnumerator0
      (if (Variables|/Game/ThirdPerson/Blueprints/BP_ThirdPersonCharacter.BP_ThirdPersonCharacter_C|GethasKey1? (Variables|Default|GetplayerRef))
        (Transformation|SetRelativeLocation (Variables|Default|GetDoor) (Math|Vector|MakeVector (- (.x _doorlocation) 1e+03) (.y _doorlocation) (.z _doorlocation)) false false :!label _label)))
    (:NewEnumerator1
      (if (Variables|/Game/ThirdPerson/Blueprints/BP_ThirdPersonCharacter.BP_ThirdPersonCharacter_C|GethasKey2? (Variables|Default|GetplayerRef))
        (goto _label)))
    (:NewEnumerator2
      (if (Variables|/Game/ThirdPerson/Blueprints/BP_ThirdPersonCharacter.BP_ThirdPersonCharacter_C|GethasKey3? (Variables|Default|GetplayerRef))
        (goto _label)))))

(event EventBeginPlay
  (Variables|Default|SetdoorLocation (Variables|/Script/Engine.SceneComponent|GetRelativeLocation (Variables|Default|GetDoor))))

(event Collision|EventActorBeginOverlap
  (params (OtherActor :type Actor%20Object%20Reference)))

(event EventTick
  (params (DeltaSeconds :type Float%20%28single-precision%29)))

(fn ConstructionScript)